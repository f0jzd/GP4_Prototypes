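; ForceFieldBP is a Chaos field actor that produces an explosion on physics objects, such as breakable Geometry Collections, within a sphere.
; Its EXPLODE event first applies external cluster strain through a radial falloff field with no attenuation to break clusters apart.
; It then applies a radial linear force, using a culling field to confine the push to the sphere.
; The Sphere component's world location and scaled radius define both fields.
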(event Custom|EXPLODE
  (bind _radialfalloff (Variables|Default|GetRadialFalloff))
  (bind _sphere (Variables|Default|GetSphere))
  (bind _returnvalue (Components|Sphere|GetScaledSphereRadius _sphere))
  (bind _returnvalue_2 (Transformation|GetWorldLocation _sphere))
  (bind _returnvalue_3 (Field|SetRadialFalloff _radialfalloff 2e+05 0.0 1.0 0.0 _returnvalue _returnvalue_2 "Field_FallOff_None"))
  (Class|FieldSystemComponent|ApplyPhysicsField (Variables|Default|GetFieldSystem) true "Field_ExternalClusterStrain" 0 _returnvalue_3)
  (Class|FieldSystemComponent|ApplyPhysicsField (Variables|Default|GetFieldSystem) true "Field_LinearForce" 0 (Field|SetCullingField (Variables|Default|GetCullingField) _returnvalue_3 (Field|SetRadialVector (Variables|Default|GetRadialVector) 1e+03 _returnvalue_2) "Field_Culling_Outside")))

(fn ConstructionScript)