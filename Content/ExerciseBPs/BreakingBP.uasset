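; BreakingBP is a Chaos field actor that applies breaking strain to destructible geometry around its Box component.
; Every Tick, it applies a linear box falloff at the box's transform as external cluster strain.
; It also submits a uniform vector, directed by the box's world location and culled by the same falloff, with physics type None.
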(event EventTick
  (params (DeltaSeconds :type Float%20%28single-precision%29))
  (bind _fieldsystem (Variables|Default|GetFieldSystem))
  (bind _boxfalloff (Variables|Default|GetBoxFalloff))
  (bind _box (Variables|Default|GetBox))
  (bind _returnvalue (Transformation|GetWorldTransform _box))
  (bind _returnvalue_2 (Field|SetBoxFalloff _boxfalloff 9e+05 0.0 1.0 0.0 _returnvalue "Field_Falloff_Linear"))
  (Class|FieldSystemComponent|ApplyPhysicsField _fieldsystem true "Field_ExternalClusterStrain" 0 _returnvalue_2)
  (Class|FieldSystemComponent|ApplyPhysicsField _fieldsystem true "Field_None" 0 (Field|SetCullingField (Variables|Default|GetCullingField) _returnvalue_2 (Field|SetUniformVector (Variables|Default|GetUniformVector) 1e+03 (Transformation|GetWorldLocation _box)) "Field_Culling_Inside")))

(fn ConstructionScript)