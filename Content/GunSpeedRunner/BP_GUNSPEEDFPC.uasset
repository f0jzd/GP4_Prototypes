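; First-person player character for GunSpeedRunner that switches between Semi, Shotgun and Sniper with number keys and handles axis-based movement and mouse look.
; Right mouse triggers the gun's movement ability: Semi launches the character upward, spending a jump charge, while Shotgun and Sniper do nothing yet.
; Tick refills two jump charges whenever the character is not falling and prints the current gun for debugging.
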(event EventTick
  (params (DeltaSeconds :type Float%20%28single-precision%29))
  (Development|PrintString (Utilities|String|EnumtoString (Variables|Default|GetGunInventory)) true true "(R=0.000000,G=0.660000,B=1.000000,A=1.000000)" 0.0)
  (if (not (AI|Components|NavMovement|IsFalling (Variables|Character|GetCharacterMovement)))
    (Variables|Default|SetJumpCount 2)))

(event Input|AxisEvents|InputAxisMoveForward/Backward
  (params (AxisValue :type Float%20%28single-precision%29))
  (bind _returnvalue (Pawn|GetControlRotation :!class /Script/Engine.Pawn))
  ;[1 1 1] MOVEMENT
  (Pawn|Input|AddMovementInput (Math|Vector|GetForwardVector (Math|Rotator|MakeRotator (.roll _returnvalue) 0.0 (.yaw _returnvalue))) AxisValue false))

(event Input|AxisEvents|InputAxisTurnRight/LeftMouse
  (params (AxisValue :type Float%20%28single-precision%29))
  ;[1 1 1] MOVEMENT
  (Pawn|Input|AddControllerYawInput AxisValue))

(event Input|AxisEvents|InputAxisLookUp/DownMouse
  (params (AxisValue :type Float%20%28single-precision%29))
  ;[1 1 1] MOVEMENT
  (Pawn|Input|AddControllerPitchInput AxisValue))

(event Input|AxisEvents|InputAxisMoveRight/Left
  (params (AxisValue :type Float%20%28single-precision%29))
  ;[1 1 1] MOVEMENT
  (Pawn|Input|AddMovementInput (Math|Vector|GetRightVector (Pawn|GetControlRotation :!class /Script/Engine.Pawn)) AxisValue false))

(event Input|MouseEvents|RightMouseButton
  (params (Key :type Key%20Structure :default "None"))
  (:Pressed
    (if (Utilities|Enum|Equal(Enum) (Variables|Default|GetGunInventory) "Semi")
      (if (> (Variables|Default|GetJumpCount) 0)
        (Character|LaunchCharacter "0,0.000000,600.000000" false true)
        (Variables|Default|SetJumpCount (- (Variables|Default|GetJumpCount) 1)))
      (elif (not (Utilities|Enum|Equal(Enum) (Variables|Default|GetGunInventory) "Shotgun"))
        (if (Utilities|Enum|Equal(Enum) (Variables|Default|GetGunInventory) "Sniper")
          _)))))

(event Input|KeyboardEvents|3
  (params (Key :type Key%20Structure :default "None"))
  (:Pressed
    (bind _output_get (Variables|Default|SetGunInventory "Sniper"))
    (Development|PrintString (Utilities|String|EnumtoString _output_get))))

(event Input|KeyboardEvents|1
  (params (Key :type Key%20Structure :default "None"))
  (:Pressed
    (bind _output_get (Variables|Default|SetGunInventory "Semi"))
    (Development|PrintString (Utilities|String|EnumtoString _output_get))))

(event Input|KeyboardEvents|2
  (params (Key :type Key%20Structure :default "None"))
  (:Pressed
    (bind _output_get (Variables|Default|SetGunInventory "Shotgun"))
    (Development|PrintString (Utilities|String|EnumtoString _output_get))))

(fn ConstructionScript)